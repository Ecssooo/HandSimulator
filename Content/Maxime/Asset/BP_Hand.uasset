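; BP_Hand is a player-controlled hand that moves along world axes and can grab, release and activate tools.
; Enhanced Input drives movement and actions, while a Sphere overlap stores the latest actor implementing BPI_Tools as grabbable.
; Grab attaches that actor to the Sphere or detaches it, depending on the CanGrab and IsGrabing flags.
; Activate sends ActivateToolMessage to the stored actor while grabbing.
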(event `self.ReceiveBeginPlay`
  (message `EnhancedInputSubsystemInterface.AddMappingContext` (pcsubsystem `EnhancedInputLocalPlayerSubsystem` (`GameplayStatics.GetPlayerController` 0)) "/Game/Maxime/Input/IMC_MHand.IMC_MHand" 0 (struct)))

(event `EnhancedInput|/Game/Maxime/Input/InputAction/IA_Move`
  (params (ActionValue :type "Vector Structure") (ElapsedSeconds :type "Float (double-precision)") (TriggeredSeconds :type "Float (double-precision)") (InputAction :type "InputAction Object Reference" :default "/Game/Maxime/Input/InputAction/IA_Move.IA_Move"))
  (:`Triggered`
    (`self.AddMovementInput` (`KismetMathLibrary.Vector_Forward`) ActionValue_X)
    (`self.AddMovementInput` (`KismetMathLibrary.Vector_Right`) ActionValue_Y)
    (`self.AddMovementInput` (`KismetMathLibrary.Vector_Up`) ActionValue_Z)))

(event `EnhancedInput|/Game/Maxime/Input/InputAction/IA_Grab`
  (params (ActionValue :type Boolean) (ElapsedSeconds :type "Float (double-precision)") (TriggeredSeconds :type "Float (double-precision)") (InputAction :type "InputAction Object Reference" :default "/Game/Maxime/Input/InputAction/IA_Grab.IA_Grab"))
  (:`Started`
    (if (`self.CanGrab`)
      (if (not (`self.IsGrabing`))
        (`self.K2_AttachToComponent` (`self.Other Actor`) (`self.Sphere`) "None" "KeepWorld" "KeepWorld" "KeepWorld" true)
        (set `self.IsGrabing` true)
        (set `self.CanGrab` false))
      (elif (`self.IsGrabing`)
        (`self.K2_DetachFromActor` (`self.Other Actor`) "KeepWorld" "KeepWorld" "KeepWorld")
        (set `self.IsGrabing` false)))))

(event `EnhancedInput|/Game/Maxime/Input/InputAction/IA_Activate`
  (params (ActionValue :type Boolean) (ElapsedSeconds :type "Float (double-precision)") (TriggeredSeconds :type "Float (double-precision)") (InputAction :type "InputAction Object Reference" :default "/Game/Maxime/Input/InputAction/IA_Activate.IA_Activate"))
  (:`Started`
    (if (`self.IsGrabing`)
      (message `/Game/Maxime/interface/BPI_Tools.ActivateTool` (`self.Other Actor`)))))

(event `self.Sphere.OnComponentBeginOverlap`
  (params (OverlappedComponent :type "PrimitiveComponent Object Reference") (OtherActor :type "Actor Object Reference") (OtherComp :type "PrimitiveComponent Object Reference") (OtherBodyIndex :type Integer) (bFromSweep :type Boolean) (SweepResult :type "HitResult Structure (by ref)"))
  (if (`KismetSystemLibrary.DoesImplementInterface` OtherActor "/Game/Maxime/interface/BPI_Tools.BPI_Tools_C")
    (set `self.CanGrab` true)
    (set `self.Other Actor` OtherActor)))

(event `self.Sphere.OnComponentEndOverlap`
  (params (OverlappedComponent :type "PrimitiveComponent Object Reference") (OtherActor :type "Actor Object Reference") (OtherComp :type "PrimitiveComponent Object Reference") (OtherBodyIndex :type Integer))
  (if (`KismetSystemLibrary.DoesImplementInterface` OtherActor "/Game/Maxime/interface/BPI_Tools.BPI_Tools_C")
    (set `self.CanGrab` false)))

(fn `UserConstructionScript`)